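; Enemy actor for a shooter that damages the hero on contact and can be killed by incoming damage.
; Overlapping a HeroBP deals damage at once and starts a looping timer that repeats it until the overlap ends.
; DecreaseHP lowers its health, and at zero it tells ShooterGameMode to decrement the enemy count and raise the score, then destroys itself.
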(event Custom|DecreaseHeroHP
  (Default|DecreaseHP (stale Collision|EventActorBeginOverlap _ashero_bp) 2e+01))

(event EventBeginPlay
  (Variables|Default|Sethp 1e+02))

(event EventDecreaseHP
  (params (amount :type Float%20%28single-precision%29))
  (bind _output_get (Variables|Default|Sethp (- (Variables|Default|Gethp) amount)))
  (if (<= _output_get 0.0)
    (bind _asshooter_game_mode (Utilities|Casting|CastToShooterGameMode (Game|GetGameMode)))
    (Default|DecreaseNumberEnemies _asshooter_game_mode)
    (bind _asshooter_game_mode_2 (Utilities|Casting|CastToShooterGameMode (Game|GetGameMode)))
    (Default|IncreaseScore _asshooter_game_mode_2)
    (Actor|DestroyActor)))

(event Collision|EventActorEndOverlap
  (params (OtherActor :type Actor%20Object%20Reference))
  (Utilities|Casting|CastToHeroBP OtherActor)
  (Utilities|Time|ClearTimerbyFunctionName 0 "DecreaseHeroHP"))

(event Collision|EventActorBeginOverlap
  (params (OtherActor :type Actor%20Object%20Reference))
  (bind _ashero_bp (Utilities|Casting|CastToHeroBP OtherActor))
  (CallFunction|DecreaseHeroHP)
  (Utilities|Time|SetTimerbyFunctionName 0 "DecreaseHeroHP" 0.3 true))

(fn ConstructionScript)