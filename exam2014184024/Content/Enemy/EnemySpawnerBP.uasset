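; Enemy spawner actor that periodically populates the level with EnemyBP AI pawns.
; On BeginPlay it caches the ShooterGameMode and starts a looping half-second timer.
; Each tick of the timer spawns an enemy at a random point inside the SpawnVolume box while the game mode's enemy count is within its cap, then increments that count.
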(event Custom|SpawnEnemy
  (bind _spawnvolume (Variables|Default|GetSpawnVolume))
  (bind _gamemode (Variables|Default|GetGameMode))
  (if (<= (Variables|/Game/ShooterGameMode.ShooterGameMode_C|GetNumberEnemies _gamemode) 10)
    (AI|SpawnAIFromClass "/Game/Enemy/EnemyBP.EnemyBP_C" 0 (Math|Random|RandomPointinBoundingBox (Transformation|GetWorldLocation _spawnvolume) (Components|Box|GetScaledBoxExtent _spawnvolume)) "0, 0, 0" false)
    (Default|IncreaseNumberEnemies _gamemode)))

(event EventBeginPlay
  (bind _asshooter_game_mode (Utilities|Casting|CastToShooterGameMode (Game|GetGameMode)))
  (Variables|Default|SetGameMode _asshooter_game_mode)
  (Utilities|Time|SetTimerbyFunctionName 0 "SpawnEnemy" 0.5 true))

(fn ConstructionScript)